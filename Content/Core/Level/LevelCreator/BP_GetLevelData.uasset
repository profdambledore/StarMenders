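; BP_GetLevelData captures the actors placed in a level into a LevelData struct for the level creator.
; StartGeneratingLevelData gathers entrance and exit door transforms, record pads, and input and output mechanics with their transforms, classes and settings.
; Input mechanics reference linked objects by name, and the result is stored in LastSavedData and returned with the given name and mesh.
; An older single-parent-class mechanic pass remains unconnected.
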(fn `StartGeneratingLevelData`
  (params (LevelStaticMesh :type "StaticMesh Object Reference") (LevelName :type Name))
  (returns (NewParam :type "LevelData Structure"))
  (locals (EntranceDoor :type "Transform Structure") (ExitDoor :type "Transform Structure") (RecordPads :type "Array of RecordPadData Structure") (InputMech :type "Array of InputMechanicData Structure") (LinkedObjects :type "Array of Name") (OutputMech :type "Array of OutputMechanicData Structure"))
  (bind _outactors (`GameplayStatics.GetAllActorsOfClass` "/Game/Core/Level/BP_LevelDoor.BP_LevelDoor_C"))
  (for _array_element _outactors
    (switch `EDoorType` (`LevelDoor.DoorType` _array_element)
      (:`Entrance`
        (bind _returnvalue (`self.GetTransform` _array_element))
        (set `local.EntranceDoor` _returnvalue))
      (:`Exit`
        (set `local.ExitDoor` _returnvalue))))
  (bind _outactors_2 (`GameplayStatics.GetAllActorsOfClass` "/Game/Core/Mechanics/BP_RecordPad.BP_RecordPad_C"))
  (for _array_element_2 _outactors_2
    (`KismetArrayLibrary.Array_Add` (`local.RecordPads`) (make `RecordPadData` (`RecordPad.RecorderIndex` _array_element_2) (`self.GetTransform` _array_element_2))))
  (bind _outactors_3 (`GameplayStatics.GetAllActorsOfClass` "/Script/StarMenders.MechanicObject_Input"))
  (for _array_element_3 _outactors_3
    (`KismetArrayLibrary.Array_Clear` (`local.LinkedObjects`))
    (for _array_element_4 _
      (`KismetArrayLibrary.Array_Add` (`local.LinkedObjects`) (`MechanicObject_Parent.ObjectName` _array_element_4)))
    (`KismetArrayLibrary.Array_Add` (`local.InputMech`) (make `InputMechanicData` (`MechanicObject_Parent.ObjectName` _array_element_3) (`self.GetTransform` _array_element_3) (`GameplayStatics.GetObjectClass` _array_element_3) (`local.LinkedObjects`))))
  (bind _outactors_4 (`GameplayStatics.GetAllActorsOfClass` "/Script/StarMenders.MechanicObject_Output"))
  (for _array_element_5 _outactors_4
    (`KismetArrayLibrary.Array_Add` (`local.OutputMech`) (make `OutputMechanicData` (`MechanicObject_Parent.ObjectName` _array_element_5) (`self.GetTransform` _array_element_5) (`GameplayStatics.GetObjectClass` _array_element_5) (`MechanicObject_Output.InputRequirement` _array_element_5) (`MechanicObject_Output.bOutputAlwaysActive` _array_element_5))))
  (bind _output_get (set `self.LastSavedData` (make `LevelData` (`local.LevelName`) (`local.LevelStaticMesh`) (`local.EntranceDoor`) (`local.ExitDoor`) (`local.RecordPads`) (`local.InputMech`) (`local.OutputMech`))))
  (return _output_get))

(fn `UserConstructionScript`)