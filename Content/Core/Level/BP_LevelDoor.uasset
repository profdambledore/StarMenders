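; BP_LevelDoor is a portal-style door that shows the view from its paired door's capture camera on its plane.
; Shortly after BeginPlay, it creates a dynamic material and viewport-sized render target, feeds the target to both that material and the paired door's camera, then calls UpdateClipPlane.
; The construction script hides both doors from its own capture camera.
; The logic setting the material's Offset parameter is unconnected.
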(event `self.ReceiveBeginPlay`
  (bind (_returnvalue_x _returnvalue_y) (`KismetMathLibrary.BreakVector2D` (`WidgetLayoutLibrary.GetViewportSize`)))
  (`KismetSystemLibrary.Delay` 0.1)
  (bind _returnvalue (`KismetMaterialLibrary.CreateDynamicMaterialInstance` "/Game/Prototype/PROTO_LevelDoorPlane.PROTO_LevelDoorPlane"))
  (bind _output_get (set `self.PortalMaterialInst` _returnvalue))
  (`PrimitiveComponent.SetMaterial` (`self.Plane`) 0 _output_get)
  (bind _returnvalue_2 (`KismetRenderingLibrary.CreateRenderTarget2D` (`KismetMathLibrary.FTrunc` _returnvalue_x) (`KismetMathLibrary.FTrunc` _returnvalue_y)))
  (bind _output_get_2 (set `self.PortalRenderTarget` _returnvalue_2))
  (`MaterialInstanceDynamic.SetTextureParameterValue` (`self.PortalMaterialInst`) "RenderTarget" _output_get_2)
  (set `SceneCaptureComponent2D.TextureTarget` (`self.PortalRenderTarget`) (`LevelDoor.CaptureCamera` (`self.PairedDoor`)))
  (`self.UpdateClipPlane`))

(fn `UserConstructionScript`
  (`SceneCaptureComponent.HideActorComponents` (`self.CaptureCamera`) self false)
  (`SceneCaptureComponent.HideActorComponents` (`self.CaptureCamera`) (`self.PairedDoor`) false))