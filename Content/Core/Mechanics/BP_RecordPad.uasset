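; BP_RecordPad is a record pad actor that displays a rotating character hologram and an energy element tinted for its recorder.
; BeginPlay restricts the RotatingMovement component to the hologram and applies one shared dynamic instance of MI_RecordPad to both meshes.
; SetupVisualElements looks up the RecorderIndex colour in ColourConsts and sets that material's colour and light multiplier.
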(event `self.ReceiveBeginPlay`
  (bind _visualelementdynamic (`self.VisualElementDynamic`))
  ;[0.01096 0.01161 0.0137] Set the RotatingMovementComponent to only rotate the Character Hologram
  (`MovementComponent.SetUpdatedComponent` (`self.RotatingMovement`) (`self.RecorderCharacterHologram`))
  (bind _returnvalue (`KismetMaterialLibrary.CreateDynamicMaterialInstance` "/Game/Core/Materials/MI_RecordPad.MI_RecordPad"))
  (set `self.VisualElementDynamic` _returnvalue)
  (`PrimitiveComponent.SetMaterial` (`self.RecorderCharacterHologram`) 0 _visualelementdynamic)
  (`PrimitiveComponent.SetMaterial` (`self.Recorder Energy Colour`) 0 _visualelementdynamic))

(event `self.SetupVisualElements`
  (bind _visualelementdynamic (`self.VisualElementDynamic`))
  (`MaterialInstanceDynamic.SetVectorParameterValue` _visualelementdynamic "Colour" (`KismetMathLibrary.Conv_ColorToLinearColor` (`BlueprintMapLibrary.Map_Find` (`self.ColourConsts`) (`self.RecorderIndex`))))
  (`MaterialInstanceDynamic.SetScalarParameterValue` _visualelementdynamic "LightMulti" 4.0))

(fn `UserConstructionScript`)