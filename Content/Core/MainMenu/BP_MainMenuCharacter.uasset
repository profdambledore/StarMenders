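; Main menu pawn that shows the menu widget with a mouse cursor and presents save slots as clickable planets.
; It async-loads the MasterSave index and sets each BP_SaveObject's planet visuals by array order, marking unused ones empty.
; A left-click release traces from the cursor; hitting a planet stores its save ID in the game instance and opens LoadingMap.
; MoveToNewState snaps the actor to a transform mapped to that menu state.
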(event `self.ReceiveBeginPlay`
  (bind _returnvalue (`|GenericCreateObject` "/Game/Core/MainMenu/WBP_MainMenu.WBP_MainMenu_C"))
  (bind _output_get (set `self.NewVar` _returnvalue))
  (`UserWidget.AddToViewport` _output_get 0)
  (set `/Game/Core/MainMenu/WBP_MainMenu.MainMenuPlayer` self _output_get)
  (bind _asplayer_controller (cast `PlayerController` (`self.GetController`)))
  (bind _output_get_2 (set `self.PC` _asplayer_controller))
  (set `PlayerController.bShowMouseCursor` true _output_get_2)
  (`self.SetupSavePlanets`))

(event `SetupSavePlanets`
  (bind _savegame (`AsyncActionHandleSaveGame.AsyncLoadGameFromSlot` "MasterSave")
    (:`Completed`
      (`/Engine/EditorBlueprintResources/StandardMacros.IsValid` _savegame
        (:`Is Valid`
          (bind _asmaster_save_game (cast `Master_SaveGame` _savegame))
          (bind _outactors (`GameplayStatics.GetAllActorsOfClass` "/Game/Core/MainMenu/BP_SaveObject.BP_SaveObject_C"))
          (for (_array_element _array_index) _outactors
            (bind _savegames (`Master_SaveGame.SaveGames` _asmaster_save_game))
            (if (`KismetArrayLibrary.Array_IsValidIndex` _savegames _array_index)
              (bind ((`SaveName` _savename) (`LastPlanet` _lastplanet)) (break `SaveData` (`|GetArrayItem` _savegames _array_index)))
              (`/Game/Core/MainMenu/BP_SaveObject.SetPlanetVisuals` _array_element _lastplanet _savename)
              (else
                (`/Game/Core/MainMenu/BP_SaveObject.SetPlanetVisuals` _array_element "EmptySave" "")))))))))

(event `Key|LeftMouseButton`
  (params (Key :type "Key Structure"))
  (bind (_worldlocation _worlddirection) (`PlayerController.DeprojectMousePositionToWorld` (`GameplayStatics.GetPlayerController` 0)))
  (:`Released`
    (bind _outhit (`KismetSystemLibrary.LineTraceSingleForObjects` _worldlocation (+ _worldlocation (* _worlddirection 20000.0)) (`|MakeArray` "ObjectTypeQuery2" :!type "EObjectTypeQuery Enum") false (`|MakeArray` self :!type "Actor Object Reference") "Persistent"))
    (bind (_bblockinghit _binitialoverlap _time _distance _location _impactpoint _normal _impactnormal _physmat _hitactor) (`GameplayStatics.BreakHitResult` _outhit))
    (if (== (`GameplayStatics.GetObjectClass` _hitactor) "/Game/Core/MainMenu/BP_SaveObject.BP_SaveObject_C")
      (bind _asbp_save_object (cast `/Game/Core/MainMenu/BP_SaveObject` _hitactor))
      (`self.LoadLevelWithSaveData` "LoadingMap" (`/Game/Core/MainMenu/BP_SaveObject.SaveID` _asbp_save_object)))))

(event `FireTraceToPlanet`)

(event `LoadLevelWithSaveData`
  (params (LevelName :type Name) (SaveData :type String))
  (bind _asparent_game_instance (cast `Parent_GameInstance` (`GameplayStatics.GetGameInstance`)))
  (set `Parent_GameInstance.CurrentSaveName` SaveData _asparent_game_instance)
  (`GameplayStatics.OpenLevel` LevelName false))

(event `MoveToNewState`
  (params (NewState :type String))
  (`self.K2_SetActorTransform` (`BlueprintMapLibrary.Map_Find` (`self.StateTransforms`) NewState)))

(fn `UserConstructionScript`)